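; BP_SMagicProjectile is a magic projectile that damages props tagged as reactive.
; Its sphere component's hit event checks only the hit actor's first tag for "ReactiveProp".
; On a match it adds a particle system, applies damage, removes its effect component and destroys itself after a short delay.
; Any other hit only draws a debug sphere and prints the actor's name, leaving the projectile alive.
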(event `self.SphereComp.OnComponentHit`
  (params (HitComponent :type "PrimitiveComponent Object Reference") (OtherActor :type "Actor Object Reference") (OtherComp :type "PrimitiveComponent Object Reference") (NormalImpulse :type "Vector Structure") (Hit :type "HitResult Structure (by ref)"))
  (bind _tags (`Actor.Tags` Hit_HitActor))
  (if (`KismetArrayLibrary.Array_IsValidIndex` _tags)
    (if (== (`|GetArrayItem` _tags) "ReactiveProp")
      (`AddComponent|NODE_AddParticleSystemComponent-0`)
      (`GameplayStatics.ApplyDamage` Hit_HitActor 20.0 null self "/Script/Engine.DamageType")
      (`ActorComponent.K2_DestroyComponent` (`self.EffectComp`))
      (`KismetSystemLibrary.Delay` 2.0)
      (`self.K2_DestroyActor`)
      (else
        (`KismetSystemLibrary.DrawDebugSphere` Hit_Location 5.0 12 (struct :`G` 0.16799 :`B` 1.0 :`A` 1.0) 1.0 1.0 :!label _label)
        (`KismetSystemLibrary.PrintString` (`KismetSystemLibrary.GetDisplayName` Hit_HitActor))))
    (else
      (goto _label))))

(fn `UserConstructionScript`)